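; Objective arrow actor that steps the player through a narrated quest: check out the trash pile, collect ammo, then get to the ship.
; Tick polls one-shot state flags to show, hide or move the arrow, update the objective and lock narration during timed audio.
; Reaching the ammo target triggers the ship stage; other stages rely on externally set flags.
; The final state hides the HUD, plays a fade-out and opens the space level.
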(event `self.ReceiveBeginPlay`
  ;[1 1 1] Remove Collision
  (`self.SetActorEnableCollision` false))

(event `self.ReceiveTick`
  (params (DeltaSeconds :type "Float (single-precision)"))
  ;[1 1 1] Arrow State One (Begin)
  (if (`self.arrowState1`)
    (set `self.arrowState1` false)
    (`self.SetActorHiddenInGame` false)
    (bind _asfirst_person_character (cast `/Game/FirstPersonBP/Blueprints/FirstPersonCharacter` (`GameplayStatics.GetPlayerCharacter` 0)))
    (set `/Game/FirstPersonBP/Blueprints/FirstPersonCharacter.NarrationLock` true _asfirst_person_character)
    (`AddComponent|NODE_AddAudioComponent-1`)
    (`KismetSystemLibrary.Delay` (`self.arrow1Delay`))
    (set `/Game/FirstPersonBP/Blueprints/FirstPersonCharacter.NarrationLock` false _asfirst_person_character)
    (set `/Game/FirstPersonBP/Blueprints/FirstPersonCharacter.CurrentObjective` "Check out the trash pile" _asfirst_person_character)
    (else
      ;[1 1 1] Arrow State 2 (Trash Pile)
      (if (`self.arrowState2`)
        (if (`self.prepareAmmoCollect`)
          (if (`self.arrowIs2`)
            (set `self.arrowIs2` false)
            (`self.SetActorHiddenInGame` true)
            (bind _asfirst_person_character_2 (cast `/Game/FirstPersonBP/Blueprints/FirstPersonCharacter` (`GameplayStatics.GetPlayerCharacter` 0)))
            (set `/Game/FirstPersonBP/Blueprints/FirstPersonCharacter.NarrationLock` true _asfirst_person_character_2)
            (`AddComponent|NODE_AddAudioComponent-3`)
            (`KismetSystemLibrary.Delay` (`self.arrow2Delay`))
            (set `/Game/FirstPersonBP/Blueprints/FirstPersonCharacter.NarrationLock` false _asfirst_person_character_2)
            (set `self.prepareAmmoCollect` false))
          (else
            (bind _asfirst_person_character_3 (cast `/Game/FirstPersonBP/Blueprints/FirstPersonCharacter` (`GameplayStatics.GetPlayerCharacter` 0)))
            (set `/Game/FirstPersonBP/Blueprints/FirstPersonCharacter.CurrentObjective` "Collect 100 ammo" _asfirst_person_character_3)
            (bind _outactors (`GameplayStatics.GetAllActorsOfClass` "/Game/FirstPersonBP/Blueprints/FirstPersonCharacter.FirstPersonCharacter_C"))
            (for _array_element _outactors
              (if (>= (`/Game/FirstPersonBP/Blueprints/FirstPersonCharacter.Ammo` _array_element) (`self.ammoToCollect`))
                (set `self.arrowState2` false)
                (set `self.arrowState3` true)))))
        (else
          ;[1 1 1] Arrow State 3 (Ammo)
          (if (`self.arrowState3`)
            (set `self.arrowState3` false)
            (`self.K2_SetActorLocation` (-10330.0 -160.0 10000.0) false true)
            (`self.SetActorHiddenInGame` false)
            (bind _asfirst_person_character_4 (cast `/Game/FirstPersonBP/Blueprints/FirstPersonCharacter` (`GameplayStatics.GetPlayerCharacter` 0)))
            (set `/Game/FirstPersonBP/Blueprints/FirstPersonCharacter.CurrentObjective` "Get to the ship" _asfirst_person_character_4)
            (set `/Game/FirstPersonBP/Blueprints/FirstPersonCharacter.NarrationLock` true _asfirst_person_character_4)
            (`AddComponent|NODE_AddAudioComponent-4`)
            (`KismetSystemLibrary.Delay` (`self.arrow3Delay`))
            (set `/Game/FirstPersonBP/Blueprints/FirstPersonCharacter.NarrationLock` false _asfirst_person_character_4)
            (else
              ;[1 1 1] Arrow State 4
              (if (`self.arrowState4`)
                (set `self.arrowState4` false)
                (`self.K2_SetActorLocation` (-10330.0 -160.0 10000.0) false true)
                (`self.SetActorHiddenInGame` true)
                (bind _asfirst_person_character_5 (cast `/Game/FirstPersonBP/Blueprints/FirstPersonCharacter` (`GameplayStatics.GetPlayerCharacter` 0)))
                (set `/Game/FirstPersonBP/Blueprints/FirstPersonCharacter.CurrentObjective` "None" _asfirst_person_character_5)
                (set `/Game/FirstPersonBP/Blueprints/FirstPersonCharacter.NarrationLock` true _asfirst_person_character_5)
                (`AddComponent|NODE_AddAudioComponent-5`)
                (`KismetSystemLibrary.Delay` (`self.arrow4Delay`))
                (set `/Game/FirstPersonBP/Blueprints/FirstPersonCharacter.NarrationLock` false _asfirst_person_character_5)
                (bind _garbagegamemanager (`/Game/Blueprints/GarbageFunctionLibrary.GetGarbageGameManager`))
                (bind _output_get (set `/Game/Blueprints/GarbageGameManager.FirstPersonHUD` (`/Game/Blueprints/GarbageGameManager.FirstPersonHUD` _garbagegamemanager) _garbagegamemanager))
                (`Widget.SetVisibility` _output_get "Hidden")
                (bind (_outactor _returnvalue) (`LevelSequencePlayer.CreateLevelSequencePlayer` "/Game/Levels/FadeOut.FadeOut"))
                (`MovieSceneSequencePlayer.Play` _returnvalue)
                (`KismetSystemLibrary.Delay` (`self.fadeOutDelay`))
                (`GameplayStatics.OpenLevelBySoftObjectPtr` "/Game/Levels/SpaceLevel.SpaceLevel")))))))))

(fn `UserConstructionScript`
  (`parent.UserConstructionScript`))