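; BP_ShipFragment is a collectible ship fragment that the first-person character picks up by touching it.
; Any overlap on its collision component adds an audio component, before the overlapping actor's class is checked.
; For an exact FirstPersonCharacter match, it hides itself and disables collision rather than being destroyed.
; It then increments the ShipFragments count on every FirstPersonCharacter in the level.
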(event `self.collisssion.OnComponentBeginOverlap`
  (params (OverlappedComponent :type "PrimitiveComponent Object Reference") (OtherActor :type "Actor Object Reference") (OtherComp :type "PrimitiveComponent Object Reference") (OtherBodyIndex :type Integer) (bFromSweep :type Boolean) (SweepResult :type "HitResult Structure (by ref)"))
  (`AddComponent|NODE_AddAudioComponent-0`)
  (if (== (`GameplayStatics.GetObjectClass` OtherActor) "/Game/FirstPersonBP/Blueprints/FirstPersonCharacter.FirstPersonCharacter_C")
    (cast `/Game/FirstPersonBP/Blueprints/FirstPersonCharacter` (`GameplayStatics.GetPlayerCharacter` 0))
    (`self.SetActorHiddenInGame` true)
    (`self.SetActorEnableCollision` false)
    (bind _outactors (`GameplayStatics.GetAllActorsOfClass` "/Game/FirstPersonBP/Blueprints/FirstPersonCharacter.FirstPersonCharacter_C"))
    (for _array_element _outactors
      (set `/Game/FirstPersonBP/Blueprints/FirstPersonCharacter.ShipFragments` (+ (`/Game/FirstPersonBP/Blueprints/FirstPersonCharacter.ShipFragments` _array_element) 1.0) _array_element))))

(fn `UserConstructionScript`)