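; BP_Ammo is an ammo pickup whose cube scales with the amount of ammo it holds.
; Its collision overlap branches on exact actor class: first-person or twin-stick projectiles increase the held amount and size, with only the former destroyed.
; A non-sneaking FirstPersonCharacter or any SpaceshipPawn hides and disables it, adding the held ammo to all actors of that class, less one for ships.
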(event `self.ReceiveBeginPlay`
  (bind _cube (`self.Cube`))
  ;[1 1 1] Begin With Size Set
  (`SceneComponent.SetWorldScale3D` _cube (+ (`SceneComponent.K2_GetComponentScale` _cube) (* (`self.AmmoHeldAmount`) (`self.SizeMultiplier`)))))

(event `self.AmmoCollisionBox.OnComponentBeginOverlap`
  (params (OverlappedComponent :type "PrimitiveComponent Object Reference") (OtherActor :type "Actor Object Reference") (OtherComp :type "PrimitiveComponent Object Reference") (OtherBodyIndex :type Integer) (bFromSweep :type Boolean) (SweepResult :type "HitResult Structure (by ref)"))
  (bind _returnvalue (`GameplayStatics.GetObjectClass` OtherActor))
  (bind _cube (`self.Cube`))
  (bind _cube_2 (`self.Cube`))
  (`|ExecutionSequence`
    (:`then_0`
      ;[1 1 1] Pick Up Ammo
      (if (== _returnvalue "/Game/FirstPersonBP/Blueprints/FirstPersonCharacter.FirstPersonCharacter_C")
        (bind _asfirst_person_character (cast `/Game/FirstPersonBP/Blueprints/FirstPersonCharacter` (`GameplayStatics.GetPlayerCharacter` 0)))
        (if (not (`/Game/FirstPersonBP/Blueprints/FirstPersonCharacter.isSneaking` _asfirst_person_character))
          (`self.SetActorHiddenInGame` true)
          (`self.SetActorEnableCollision` false)
          (bind _outactors (`GameplayStatics.GetAllActorsOfClass` "/Game/FirstPersonBP/Blueprints/FirstPersonCharacter.FirstPersonCharacter_C"))
          (for _array_element _outactors
            (set `/Game/FirstPersonBP/Blueprints/FirstPersonCharacter.Ammo` (+ (`/Game/FirstPersonBP/Blueprints/FirstPersonCharacter.Ammo` _array_element) (`KismetMathLibrary.Conv_IntToDouble` (`self.AmmoHeldAmount`))) _array_element)))))
    (:`then_1`
      ;[1 1 1] Bullet Hits Ammo
      (if (== _returnvalue "/Game/FirstPersonBP/Blueprints/FirstPersonProjectile.FirstPersonProjectile_C")
        (`self.K2_DestroyActor` OtherActor) ; Then destroy this projectile
        (set `self.AmmoHeldAmount` (+ (`self.AmmoHeldAmount`) 1))
        (`SceneComponent.SetWorldScale3D` _cube (+ (`SceneComponent.K2_GetComponentScale` _cube) (* (`self.AmmoHeldAmount`) (`self.SizeMultiplier`))))))
    (:`then_2`
      ;[1 1 1] Ship Bullet Hits Ammo
      (if (== _returnvalue "/Game/TwinStickBP/Blueprints/TwinStickProjectile.TwinStickProjectile_C")
        (set `self.AmmoHeldAmount` (+ (`self.AmmoHeldAmount`) 1))
        (`SceneComponent.SetWorldScale3D` _cube_2 (+ (`SceneComponent.K2_GetComponentScale` _cube_2) (* (`self.AmmoHeldAmount`) (`self.SizeMultiplier`))))))
    (:`then_3`
      ;[1 1 1] Pick Up Ammo
      (if (== _returnvalue "/Game/TwinStickBP/Blueprints/SpaceshipPawn.SpaceshipPawn_C")
        (`self.SetActorHiddenInGame` true)
        (`self.SetActorEnableCollision` false)
        (bind _outactors_2 (`GameplayStatics.GetAllActorsOfClass` "/Game/TwinStickBP/Blueprints/SpaceshipPawn.SpaceshipPawn_C"))
        (for _array_element_2 _outactors_2
          (set `/Game/TwinStickBP/Blueprints/SpaceshipPawn.Ammo` (- (+ (`/Game/TwinStickBP/Blueprints/SpaceshipPawn.Ammo` _array_element_2) (`KismetMathLibrary.Conv_IntToDouble` (`self.AmmoHeldAmount`))) 1.0) _array_element_2))))))

(fn `UserConstructionScript`)