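; BP_TriggerStart is a starting trigger that switches on the first state flag of every BP_Arrow in the level.
; Its three collision components share one overlap sequence, which hides the trigger and disables its collision if the overlapping actor is the FirstPersonCharacter.
; The sequence's second branch sets ArrowState1 on all arrows found by class lookup, outside that character check.
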(event `self.Collision.OnComponentBeginOverlap`
  (params (OverlappedComponent :type "PrimitiveComponent Object Reference") (OtherActor :type "Actor Object Reference") (OtherComp :type "PrimitiveComponent Object Reference") (OtherBodyIndex :type Integer) (bFromSweep :type Boolean) (SweepResult :type "HitResult Structure (by ref)"))
  ;[1 1 1] Starting Trigger
  (`|ExecutionSequence` :!label _label
    (:`then_0`
      (if (== (`GameplayStatics.GetObjectClass` OtherActor) "/Game/FirstPersonBP/Blueprints/FirstPersonCharacter.FirstPersonCharacter_C")
        (`self.SetActorHiddenInGame` true)
        (`self.SetActorEnableCollision` false)))
    (:`then_1`
      (bind _outactors (`GameplayStatics.GetAllActorsOfClass` "/Game/Blueprints/BP_Arrow.BP_Arrow_C"))
      (for _array_element _outactors
        (set `/Game/Blueprints/BP_Arrow.arrowState1` true _array_element)))))

(event `self.Collision2.OnComponentBeginOverlap`
  (params (OverlappedComponent :type "PrimitiveComponent Object Reference") (OtherActor :type "Actor Object Reference") (OtherComp :type "PrimitiveComponent Object Reference") (OtherBodyIndex :type Integer) (bFromSweep :type Boolean) (SweepResult :type "HitResult Structure (by ref)"))
  ;[1 1 1] Starting Trigger
  (goto _label))

(event `self.Collision1.OnComponentBeginOverlap`
  (params (OverlappedComponent :type "PrimitiveComponent Object Reference") (OtherActor :type "Actor Object Reference") (OtherComp :type "PrimitiveComponent Object Reference") (OtherBodyIndex :type Integer) (bFromSweep :type Boolean) (SweepResult :type "HitResult Structure (by ref)"))
  ;[1 1 1] Starting Trigger
  (goto _label))

(fn `UserConstructionScript`)