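; Asteroid actor that damages the spaceship on overlap and breaks apart when touched by the ship or a TwinStickProjectile.
; BeginPlay randomizes its material and PainAmount, which also drives its added scale.
; A ship overlap subtracts PainAmount from every SpaceshipPawn's health.
; Breaking spawns a BP_BrokenAsteroid with matching piece materials, then hides the asteroid and disables collision rather than destroying it.
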(event `self.ReceiveBeginPlay`
  (bind _sphere (`self.Sphere`))
  (bind _sphere_2 (`self.Sphere`))
  (`|ExecutionSequence`
    (:`then_0`
      ;[1 1 1] Set Material
      (if (`KismetMathLibrary.RandomBool`)
        (if (`KismetMathLibrary.RandomBool`)
          (`PrimitiveComponent.SetMaterial` _sphere_2 0 "/Game/Materials/Garbage.Garbage")
          (set `self.CurrentMaterial` 1)
          (else
            (`PrimitiveComponent.SetMaterial` _sphere_2 0 "/Game/StarterContent/Props/Materials/M_Rock.M_Rock")
            (set `self.CurrentMaterial` 2)))
        (elif (`KismetMathLibrary.RandomBool`)
          (`PrimitiveComponent.SetMaterial` _sphere_2 0 "/Game/StarterContent/Materials/M_Rock_Slate.M_Rock_Slate")
          (set `self.CurrentMaterial` 3)
          (else
            (`PrimitiveComponent.SetMaterial` _sphere_2 0 "/Game/Materials/Garbage.Garbage")
            (set `self.CurrentMaterial` 1)))))
    (:`then_1`
      ;[1 1 1] Set Pain Amount
      (if (`KismetMathLibrary.RandomBool`)
        (if (`KismetMathLibrary.RandomBool`)
          (if (`KismetMathLibrary.RandomBool`)
            (set `self.PainAmount` 0.05)
            (else
              (set `self.PainAmount` 0.05)))
          (elif (`KismetMathLibrary.RandomBool`)
            (set `self.PainAmount` 0.1)
            (else
              (set `self.PainAmount` 0.2))))
        (elif (`KismetMathLibrary.RandomBool`)
          (if (`KismetMathLibrary.RandomBool`)
            (set `self.PainAmount` 0.3)
            (else
              (set `self.PainAmount` 0.4)))
          (elif (`KismetMathLibrary.RandomBool`)
            (set `self.PainAmount` 0.5)
            (else
              (set `self.PainAmount` 0.6))))))
    (:`then_2`
      ;[1 1 1] Set Scale
      (`SceneComponent.SetWorldScale3D` _sphere (+ (`SceneComponent.K2_GetComponentScale` _sphere) (* (`self.PainAmount`) (`self.SizeMultiplier`)))))))

(event `self.Sphere1.OnComponentBeginOverlap`
  (params (OverlappedComponent :type "PrimitiveComponent Object Reference") (OtherActor :type "Actor Object Reference") (OtherComp :type "PrimitiveComponent Object Reference") (OtherBodyIndex :type Integer) (bFromSweep :type Boolean) (SweepResult :type "HitResult Structure (by ref)"))
  (bind _returnvalue (`GameplayStatics.GetObjectClass` OtherActor))
  ;[1 1 1] Detect Touch
  (if (== _returnvalue "/Game/TwinStickBP/Blueprints/SpaceshipPawn.SpaceshipPawn_C")
    (`|ExecutionSequence`
      (:`then_0`
        ;[1 1 1] Damage Upon Touch
        (bind _outactors (`GameplayStatics.GetAllActorsOfClass` "/Game/TwinStickBP/Blueprints/SpaceshipPawn.SpaceshipPawn_C"))
        (for _array_element _outactors
          (set `/Game/TwinStickBP/Blueprints/SpaceshipPawn.SpaceshipHealth` (- (`/Game/TwinStickBP/Blueprints/SpaceshipPawn.SpaceshipHealth` _array_element) (`self.PainAmount`)) _array_element)))
      (:`then_1`
        ;[1 1 1] Break Asteroid Upon Touch
        (bind _returnvalue_2 (`|SpawnActorFromClass` "/Game/Blueprints/Asteroid/BP_BrokenAsteroid.BP_BrokenAsteroid_C" (`SceneComponent.K2_GetComponentToWorld` (`self.Sphere`)) "AlwaysSpawn" "OverrideRootScale" null null :!label _label))
        (`self.SetActorEnableCollision` false)
        (`self.SetActorHiddenInGame` true)
        (if (== (`self.CurrentMaterial`) 1)
          (`PrimitiveComponent.SetMaterial` (`/Game/Blueprints/Asteroid/BP_BrokenAsteroid.Sphere_001` _returnvalue_2) 0 "/Game/Materials/Garbage.Garbage")
          (`PrimitiveComponent.SetMaterial` (`/Game/Blueprints/Asteroid/BP_BrokenAsteroid.Sphere_002` _returnvalue_2) 0 "/Game/Materials/Garbage.Garbage")
          (`PrimitiveComponent.SetMaterial` (`/Game/Blueprints/Asteroid/BP_BrokenAsteroid.Sphere_003` _returnvalue_2) 0 "/Game/Materials/Garbage.Garbage")
          (`PrimitiveComponent.SetMaterial` (`/Game/Blueprints/Asteroid/BP_BrokenAsteroid.Sphere` _returnvalue_2) 0 "/Game/Materials/Garbage.Garbage")
          (`PrimitiveComponent.SetMaterial` (`/Game/Blueprints/Asteroid/BP_BrokenAsteroid.Sphere_004` _returnvalue_2) 0 "/Game/Materials/Garbage.Garbage")
          (`PrimitiveComponent.SetMaterial` (`/Game/Blueprints/Asteroid/BP_BrokenAsteroid.Sphere_005` _returnvalue_2) 0 "/Game/Materials/Garbage.Garbage")
          (`PrimitiveComponent.SetMaterial` (`/Game/Blueprints/Asteroid/BP_BrokenAsteroid.Sphere_006` _returnvalue_2) 0 "/Game/Materials/Garbage.Garbage")
          (`PrimitiveComponent.SetMaterial` (`/Game/Blueprints/Asteroid/BP_BrokenAsteroid.Sphere_007` _returnvalue_2) 0 "/Game/Materials/Garbage.Garbage")
          (`KismetSystemLibrary.Delay` (`self.Duration`) :!label _label_2)
          (`self.SetActorEnableCollision` false)
          (`self.SetActorHiddenInGame` true)
          (elif (== (`self.CurrentMaterial`) 2)
            (bind _sphere (`/Game/Blueprints/Asteroid/BP_BrokenAsteroid.Sphere` _returnvalue_2))
            (`PrimitiveComponent.SetMaterial` _sphere 0 "/Game/StarterContent/Props/Materials/M_Rock.M_Rock")
            (`PrimitiveComponent.SetMaterial` (`/Game/Blueprints/Asteroid/BP_BrokenAsteroid.Sphere_001` _returnvalue_2) 0 "/Game/StarterContent/Props/Materials/M_Rock.M_Rock")
            (`PrimitiveComponent.SetMaterial` (`/Game/Blueprints/Asteroid/BP_BrokenAsteroid.Sphere_002` _returnvalue_2) 0 "/Game/StarterContent/Props/Materials/M_Rock.M_Rock")
            (`PrimitiveComponent.SetMaterial` (`/Game/Blueprints/Asteroid/BP_BrokenAsteroid.Sphere_003` _returnvalue_2) 0 "/Game/StarterContent/Props/Materials/M_Rock.M_Rock")
            (`PrimitiveComponent.SetMaterial` (`/Game/Blueprints/Asteroid/BP_BrokenAsteroid.Sphere_004` _returnvalue_2) 0 "/Game/StarterContent/Props/Materials/M_Rock.M_Rock")
            (`PrimitiveComponent.SetMaterial` (`/Game/Blueprints/Asteroid/BP_BrokenAsteroid.Sphere_005` _returnvalue_2) 0 "/Game/StarterContent/Props/Materials/M_Rock.M_Rock")
            (`PrimitiveComponent.SetMaterial` (`/Game/Blueprints/Asteroid/BP_BrokenAsteroid.Sphere_006` _returnvalue_2) 0 "/Game/StarterContent/Props/Materials/M_Rock.M_Rock")
            (`PrimitiveComponent.SetMaterial` (`/Game/Blueprints/Asteroid/BP_BrokenAsteroid.Sphere_007` _returnvalue_2) 0 "/Game/StarterContent/Props/Materials/M_Rock.M_Rock")
            (goto _label_2)
            (elif (== (`self.CurrentMaterial`) 3)
              (`PrimitiveComponent.SetMaterial` _sphere 0 "/Game/StarterContent/Materials/M_Rock_Slate.M_Rock_Slate")
              (`PrimitiveComponent.SetMaterial` (`/Game/Blueprints/Asteroid/BP_BrokenAsteroid.Sphere_001` _returnvalue_2) 0 "/Game/StarterContent/Materials/M_Rock_Slate.M_Rock_Slate")
              (`PrimitiveComponent.SetMaterial` (`/Game/Blueprints/Asteroid/BP_BrokenAsteroid.Sphere_002` _returnvalue_2) 0 "/Game/StarterContent/Materials/M_Rock_Slate.M_Rock_Slate")
              (`PrimitiveComponent.SetMaterial` (`/Game/Blueprints/Asteroid/BP_BrokenAsteroid.Sphere_003` _returnvalue_2) 0 "/Game/StarterContent/Materials/M_Rock_Slate.M_Rock_Slate")
              (`PrimitiveComponent.SetMaterial` (`/Game/Blueprints/Asteroid/BP_BrokenAsteroid.Sphere_004` _returnvalue_2) 0 "/Game/StarterContent/Materials/M_Rock_Slate.M_Rock_Slate")
              (`PrimitiveComponent.SetMaterial` (`/Game/Blueprints/Asteroid/BP_BrokenAsteroid.Sphere_005` _returnvalue_2) 0 "/Game/StarterContent/Materials/M_Rock_Slate.M_Rock_Slate")
              (`PrimitiveComponent.SetMaterial` (`/Game/Blueprints/Asteroid/BP_BrokenAsteroid.Sphere_006` _returnvalue_2) 0 "/Game/StarterContent/Materials/M_Rock_Slate.M_Rock_Slate")
              (`PrimitiveComponent.SetMaterial` (`/Game/Blueprints/Asteroid/BP_BrokenAsteroid.Sphere_007` _returnvalue_2) 0 "/Game/StarterContent/Materials/M_Rock_Slate.M_Rock_Slate")
              (goto _label_2))))))
    (elif (== _returnvalue "/Game/TwinStickBP/Blueprints/TwinStickProjectile.TwinStickProjectile_C")
      (goto _label))))

(fn `UserConstructionScript`)