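; BP_ShipTriggerSpace is a one-shot trigger volume that advances the guide arrows and saves player ammo.
; The first ShipCollision overlap clears CanTouch, even if the overlapping actor is not the player.
; For an exact FirstPersonCharacter match, it sets ArrowState4 on every BP_Arrow.
; Inside that arrow loop, it copies each FirstPersonCharacter's Ammo into GarbageGameInstance's AmmoGameInstance.
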(event `self.ShipCollision.OnComponentBeginOverlap`
  (params (OverlappedComponent :type "PrimitiveComponent Object Reference") (OtherActor :type "Actor Object Reference") (OtherComp :type "PrimitiveComponent Object Reference") (OtherBodyIndex :type Integer) (bFromSweep :type Boolean) (SweepResult :type "HitResult Structure (by ref)"))
  ;[1 1 1] Trigger Arrow 4
  (if (`self.canTouch`)
    (set `self.canTouch` false)
    (if (== (`GameplayStatics.GetObjectClass` OtherActor) "/Game/FirstPersonBP/Blueprints/FirstPersonCharacter.FirstPersonCharacter_C")
      (bind _outactors (`GameplayStatics.GetAllActorsOfClass` "/Game/Blueprints/BP_Arrow.BP_Arrow_C"))
      (for _array_element _outactors
        (set `/Game/Blueprints/BP_Arrow.arrowState4` true _array_element)
        (bind _outactors_2 (`GameplayStatics.GetAllActorsOfClass` "/Game/FirstPersonBP/Blueprints/FirstPersonCharacter.FirstPersonCharacter_C"))
        (for _array_element_2 _outactors_2
          (bind _asgarbage_game_instance (cast `/Game/Blueprints/GarbageGameInstance` (`GameplayStatics.GetGameInstance`)))
          (set `/Game/Blueprints/GarbageGameInstance.Ammo(GameInstance)` (`/Game/FirstPersonBP/Blueprints/FirstPersonCharacter.Ammo` _array_element_2) _asgarbage_game_instance))))))

(fn `UserConstructionScript`)