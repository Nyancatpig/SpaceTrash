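; Game manager that controls the game's Running, Won, Lost and Abandon states with their HUDs.
; Init has the game mode create the UI, then SetState shows the level-specific HUD while Running, or an end or menu screen with mouse and pause.
; On PlanetLevel, BeginPlay holds the player's narration lock for a delay, then sets the objective.
; ResetGame reopens CityLevel and restores game instance ammo.
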(event `self.ReceiveBeginPlay`
  (bind _returnvalue (`GameplayStatics.GetCurrentLevelName` true))
  (if (`KismetStringLibrary.EqualEqual_StrStr` _returnvalue "PlanetLevel")
    (bind _asfirst_person_character (cast `/Game/FirstPersonBP/Blueprints/FirstPersonCharacter` (`GameplayStatics.GetPlayerCharacter` 0)))
    (set `/Game/FirstPersonBP/Blueprints/FirstPersonCharacter.NarrationLock` true _asfirst_person_character)
    (`KismetSystemLibrary.Delay` (`self.Duration`))
    (set `/Game/FirstPersonBP/Blueprints/FirstPersonCharacter.NarrationLock` false _asfirst_person_character)
    (set `/Game/FirstPersonBP/Blueprints/FirstPersonCharacter.CurrentObjective` "Find the missing pieces" _asfirst_person_character)))

(fn `Get State`
  (returns (State :type "/Game/HUD/E_GarbageGameStates Enum"))
  (return (`self.Current Game State`)))

(fn `Init`
  (bind _asgarbage_game_mode (cast `/Game/Levels/GarbageGameMode` (`GameplayStatics.GetGameMode`)))
  (`/Game/Levels/GarbageGameMode.CreateUI` _asgarbage_game_mode)
  (`self.Set State` "NewEnumerator0"))

(fn `Reset Game`
  (`GameplayStatics.OpenLevelBySoftObjectPtr` "/Game/Levels/CityLevel.CityLevel")
  (bind _asgarbage_game_instance (cast `/Game/Blueprints/GarbageGameInstance` (`GameplayStatics.GetGameInstance`)))
  (set `/Game/Blueprints/GarbageGameInstance.Ammo(GameInstance)` 5.0 _asgarbage_game_instance))

(fn `Set State`
  (params (CurrentGameState :type "/Game/HUD/E_GarbageGameStates Enum" :default "NewEnumerator0"))
  (if (`|EnumInequality` CurrentGameState (`self.Current Game State`))
    (`/Game/Blueprints/GarbageFunctionLibrary.HideUI`)
    (bind _output_get (set `self.Current Game State` CurrentGameState))
    (switch `/Game/HUD/E_GarbageGameStates` _output_get
      (:`NewEnumerator0`
        (bind _returnvalue (`GameplayStatics.GetCurrentLevelName` true))
        (if (`KismetStringLibrary.EqualEqual_StrStr` _returnvalue "CityLevel")
          (`Widget.SetVisibility` (`self.FirstPersonHUD`) "Visible")
          (`/Game/Blueprints/GarbageFunctionLibrary.Show Mouse` false :!label _label)
          (else
            (bind _returnvalue_2 (`GameplayStatics.GetCurrentLevelName` true))
            (if (`KismetStringLibrary.EqualEqual_StrStr` _returnvalue_2 "SpaceLevel")
              (`Widget.SetVisibility` (`self.SpaceHUD`) "Visible")
              (goto _label)
              (else
                (bind _returnvalue_3 (`GameplayStatics.GetCurrentLevelName` true))
                (if (`KismetStringLibrary.EqualEqual_StrStr` _returnvalue_3 "PlanetLevel")
                  (`Widget.SetVisibility` (`self.FirstPersonHUD`) "Visible")
                  (goto _label)
                  (else
                    (bind _returnvalue_4 (`GameplayStatics.GetCurrentLevelName` true))
                    (if (`KismetStringLibrary.EqualEqual_StrStr` _returnvalue_4 "GlobeLevel")
                      (`Widget.SetVisibility` (`self.FirstPersonHUD`) "Visible")
                      (goto _label)))))))))
      (:`NewEnumerator1`
        (`Widget.SetVisibility` (`self.WonHUD`) "Visible")
        (`/Game/Blueprints/GarbageFunctionLibrary.Show Mouse` true :!label _label_2)
        (`GameplayStatics.SetGamePaused` true))
      (:`NewEnumerator2`
        (`Widget.SetVisibility` (`self.LooseHUD`) "Visible")
        (goto _label_2))
      (:`NewEnumerator3`
        (`Widget.SetVisibility` (`self.MenuHUD`) "Visible")
        (goto _label_2)))))

(fn `UserConstructionScript`)