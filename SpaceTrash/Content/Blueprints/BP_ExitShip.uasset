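; BP_ExitShip is the level exit ship, hidden and non-collidable until the player's ShipFragments count reaches 29.
; Tick polls that count, reveals the mesh, clears the objective, and plays one-time narration under NarrationLock before arming the Rrrrrr trigger.
; Player overlap plays closing narration and a FadeOut sequence, saves ammo to GarbageGameInstance, then opens GlobeLevel.
; Fixed Delays time both narrations and the transition.
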(event `self.ReceiveBeginPlay`
  (bind _staticmeshcomponent (`self.StaticMeshComponent`))
  (`SceneComponent.SetVisibility` _staticmeshcomponent false false)
  (`PrimitiveComponent.SetCollisionEnabled` _staticmeshcomponent "NoCollision")
  (`PrimitiveComponent.SetCollisionEnabled` (`self.rrrrrr`) "NoCollision"))

(event `self.ReceiveTick`
  (params (DeltaSeconds :type "Float (single-precision)"))
  (bind _staticmeshcomponent (`self.StaticMeshComponent`))
  (bind _asfirst_person_character (cast `/Game/FirstPersonBP/Blueprints/FirstPersonCharacter` (`GameplayStatics.GetPlayerCharacter` 0)))
  (if (== (`/Game/FirstPersonBP/Blueprints/FirstPersonCharacter.ShipFragments` _asfirst_person_character) 29.0)
    (`SceneComponent.SetVisibility` _staticmeshcomponent true false)
    (`PrimitiveComponent.SetCollisionEnabled` _staticmeshcomponent "QueryAndPhysics")
    (if (not (`self.isSpeaking`))
      (set `/Game/FirstPersonBP/Blueprints/FirstPersonCharacter.CurrentObjective` "None" _asfirst_person_character)
      (set `/Game/FirstPersonBP/Blueprints/FirstPersonCharacter.NarrationLock` true _asfirst_person_character)
      (set `self.isSpeaking` true)
      (`AddComponent|NODE_AddAudioComponent-3`)
      (`KismetSystemLibrary.Delay` 6.0)
      (set `/Game/FirstPersonBP/Blueprints/FirstPersonCharacter.NarrationLock` false _asfirst_person_character)
      (`PrimitiveComponent.SetCollisionEnabled` (`self.rrrrrr`) "QueryAndPhysics"))))

(event `self.rrrrrr.OnComponentBeginOverlap`
  (params (OverlappedComponent :type "PrimitiveComponent Object Reference") (OtherActor :type "Actor Object Reference") (OtherComp :type "PrimitiveComponent Object Reference") (OtherBodyIndex :type Integer) (bFromSweep :type Boolean) (SweepResult :type "HitResult Structure (by ref)"))
  (if (== (`GameplayStatics.GetObjectClass` OtherActor) "/Game/FirstPersonBP/Blueprints/FirstPersonCharacter.FirstPersonCharacter_C")
    (`self.SetActorEnableCollision` false)
    (bind _asfirst_person_character (cast `/Game/FirstPersonBP/Blueprints/FirstPersonCharacter` (`GameplayStatics.GetPlayerCharacter` 0)))
    (set `/Game/FirstPersonBP/Blueprints/FirstPersonCharacter.NarrationLock` true _asfirst_person_character)
    (`AddComponent|NODE_AddAudioComponent-4`)
    (`KismetSystemLibrary.Delay` 9.0)
    (set `/Game/FirstPersonBP/Blueprints/FirstPersonCharacter.NarrationLock` false _asfirst_person_character)
    (bind (_outactor _returnvalue) (`LevelSequencePlayer.CreateLevelSequencePlayer` "/Game/Levels/FadeOut.FadeOut"))
    (`MovieSceneSequencePlayer.Play` _returnvalue)
    (`KismetSystemLibrary.Delay` (`self.fadeOutDelay`))
    (bind _asgarbage_game_instance (cast `/Game/Blueprints/GarbageGameInstance` (`GameplayStatics.GetGameInstance`)))
    (bind _asfirst_person_character_2 (cast `/Game/FirstPersonBP/Blueprints/FirstPersonCharacter` (`GameplayStatics.GetPlayerCharacter` 0)))
    (set `/Game/Blueprints/GarbageGameInstance.Ammo(GameInstance)` (`/Game/FirstPersonBP/Blueprints/FirstPersonCharacter.Ammo` _asfirst_person_character_2) _asgarbage_game_instance)
    (`GameplayStatics.OpenLevelBySoftObjectPtr` "/Game/Levels/GlobeLevel.GlobeLevel")))

(fn `UserConstructionScript`)